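; Construction-script actor that scatters instances of a mesh inside a box-shaped spawn area.
; Each construction run clears the instanced mesh component, reads the box's scaled extents, then adds the configured number of instances.
; A helper places each one at a random X/Y within those extents with random yaw, drawn from a random stream, leaving local Z at zero.
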(fn `SpawnInstanceAtRandomPoint`
  (params (InstancingComponent :type "InstancedStaticMeshComponent Object Reference") (SpawnAreaExtents :type "Vector Structure"))
  (bind (_returnvalue_x _returnvalue_y) (`KismetMathLibrary.BreakVector` (* SpawnAreaExtents (-1.0 -1.0 -1.0))))
  (bind _randomstream (`self.RandomStream`))
  (bind (_returnvalue_roll _returnvalue_pitch _returnvalue_yaw) (`KismetMathLibrary.BreakRotator` (`KismetMathLibrary.RandomRotatorFromStream` _randomstream)))
  (`InstancedStaticMeshComponent.AddInstance` InstancingComponent (`KismetMathLibrary.MakeTransform` (`KismetMathLibrary.MakeVector` (`KismetMathLibrary.RandomFloatInRangeFromStream` _randomstream _returnvalue_x (.x SpawnAreaExtents)) (`KismetMathLibrary.RandomFloatInRangeFromStream` _randomstream _returnvalue_y (.y SpawnAreaExtents))) (`KismetMathLibrary.MakeRotator` 0.0 0.0 _returnvalue_yaw)) false))

(fn `UserConstructionScript`
  (locals (SpawnAreaExtents :type "Vector Structure"))
  (`|ExecutionSequence`
    (:`then_0`
      (`InstancedStaticMeshComponent.ClearInstances` (`self.InstancedMesh`)))
    (:`then_1`
      (set `local.SpawnAreaExtents` (`BoxComponent.GetScaledBoxExtent` (`self.SpawnArea`))))
    (:`then_2`
      (for _ (range (`self.NumInstances`))
        (`self.SpawnInstanceAtRandomPoint` (`self.InstancedMesh`) (`local.SpawnAreaExtents`))))))